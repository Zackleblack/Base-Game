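; Battery pickup actor that adds a battery to the first-person player's held count when touched.
; On BeginPlay it casts and caches the player character as BP_TestFirstPerson.
; When that player overlaps the collision sphere, it increments BatteriesHeld with a clamped cap, calls the player's update for the count and destroys itself, even if the count is already full.
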(event `self.ReceiveBeginPlay`
  (bind _asbp_test_first_person (cast `/Game/Developer/ZackStuff/Blueprints/BP_TestFirstPerson` (`GameplayStatics.GetPlayerCharacter` 0)))
  (set `self.Player Reference` _asbp_test_first_person))

(event `self.SphereColision.OnComponentBeginOverlap`
  (params (OverlappedComponent :type "PrimitiveComponent Object Reference") (OtherActor :type "Actor Object Reference") (OtherComp :type "PrimitiveComponent Object Reference") (OtherBodyIndex :type Integer) (bFromSweep :type Boolean) (SweepResult :type "HitResult Structure (by ref)"))
  (bind _player_reference (`self.Player Reference`))
  (if (== OtherActor (`self.Player Reference`))
    (set `/Game/Developer/ZackStuff/Blueprints/BP_TestFirstPerson.BatteriesHeld` (`KismetMathLibrary.Clamp` (+ (`/Game/Developer/ZackStuff/Blueprints/BP_TestFirstPerson.BatteriesHeld` _player_reference) 1) 0 10) _player_reference)
    (`/Game/Developer/ZackStuff/Blueprints/BP_TestFirstPerson.UpdateBatteriesHeld` (`self.Player Reference`))
    (`self.K2_DestroyActor`)))

(fn `UserConstructionScript`)